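; BP_Guard is a guard Blueprint that checks whether the player carries the correct password.
; On BeginPlay it casts player 0's character to BP_ThirdPersonCharacter and caches the reference.
; The CheckPlayerPassword event compares its own ThePassWord with the player's PassWord and prints a green True or red False.
; Nothing in this graph calls that event, and the overlap and Tick events are empty.
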(event `self.ReceiveBeginPlay`
  (bind _asbp_third_person_character (cast `/Game/ThirdPerson/Blueprints/BP_ThirdPersonCharacter` (`GameplayStatics.GetPlayerCharacter` 0)))
  (set `self.Player Ref` _asbp_third_person_character))

(event `Check Player Password`
  (if (`KismetTextLibrary.EqualEqual_TextText` (`self.The PassWord`) (`/Game/ThirdPerson/Blueprints/BP_ThirdPersonCharacter.PassWord` (`self.Player Ref`)))
    (`KismetSystemLibrary.PrintString` "True" true true (struct :`G` 1.0 :`B` 0.440505 :`A` 1.0))
    (else
      (`KismetSystemLibrary.PrintString` "False" true true (struct :`R` 0.505208 :`G` 0.009844 :`A` 1.0)))))

(fn `UserConstructionScript`)