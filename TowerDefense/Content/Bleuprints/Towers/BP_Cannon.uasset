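; BP_Cannon is a tower that automatically fires cannonballs at enemies crossing its line of fire.
; Each Tick it line-traces 2500 units along its Arrow component, with persistent debug drawing, and triggers ShootEvent on hitting a BP_EnemiParent.
; A CanShoot flag and a FireRate delay throttle firing.
; Shoot plays an explosion sound and muzzle effect, then spawns a BP_CannonBall at the Arrow, facing forward.
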(event `self.ReceiveBeginPlay`)

(event `self.ReceiveTick`
  (params (DeltaSeconds :type "Float (single-precision)"))
  (bind _arrow (`self.Arrow`))
  (bind _returnvalue (`SceneComponent.K2_GetComponentLocation` _arrow))
  (bind _outhit (`KismetSystemLibrary.LineTraceSingle` :`Start` _returnvalue :`End` (+ _returnvalue (* (`KismetMathLibrary.GetForwardVector` (`SceneComponent.K2_GetComponentRotation` _arrow)) 2500.0)) :`TraceChannel` "TraceTypeQuery1" :`DrawDebugType` "Persistent"))
  (cast `/Game/Bleuprints/Enemies/BP_EnemiParent` (`.HitActor` (`GameplayStatics.BreakHitResult` _outhit)))
  (`self.Shoot Event`))

(event `Shoot Event`
  (if (`self.Can Shoot`)
    (set `self.Can Shoot` false)
    (`self.Shoot`)
    (`KismetSystemLibrary.Delay` (`self.Fire Rate`))
    (set `self.Can Shoot` true)))

(fn `Shoot`
  (bind _arrow (`self.Arrow`))
  (bind _arrow_2 (`self.Arrow`))
  (bind _returnvalue_location (`KismetMathLibrary.BreakTransform` (`SceneComponent.K2_GetComponentToWorld` _arrow)))
  (bind _returnvalue_location_2 (`KismetMathLibrary.BreakTransform` (`SceneComponent.K2_GetComponentToWorld` _arrow_2)))
  (`GameplayStatics.PlaySoundAtLocation` "/Game/StarterContent/Audio/Explosion01.Explosion01" _returnvalue_location (struct) 1.0 1.0 0.0 null null null null)
  (`GameplayStatics.SpawnEmitterAtLocation` "/Game/Polygon/PolygonPirates/ParticleFX/P_FX_Cannon_Fire.P_FX_Cannon_Fire" _returnvalue_location (`KismetMathLibrary.Conv_VectorToRotator` (`SceneComponent.GetForwardVector` _arrow)))
  (`|SpawnActorFromClass` "/Game/Bleuprints/Projectiles/BP_CannonBall.BP_CannonBall_C" (`KismetMathLibrary.MakeTransform` _returnvalue_location_2 (`KismetMathLibrary.Conv_VectorToRotator` (`SceneComponent.GetForwardVector` _arrow_2))) "Undefined" "OverrideRootScale" null null))

(fn `UserConstructionScript`)