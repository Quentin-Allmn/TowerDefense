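; Druid Soothsayer tower that tracks enemies in range and is set up to fire spells at them.
; Its collision sphere maintains an in-range list, from which SelectTarget picks a random target.
; Gated events form aim and reset loops, but the rotation and timed-fire logic is disconnected and reset handlers are empty.
; Shoot spawns BP_Devin_Spell at the Arrow, but only that unreached logic calls it.
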(event `self.ReceiveBeginPlay`
  (bind _asbp_player (cast `/Game/Bleuprints/Player/BP_Player` (`GameplayStatics.GetPlayerCharacter` 0)))
  (set `self.Player Ref` _asbp_player))

(event `self.ReceiveActorBeginOverlap`
  (params (OtherActor :type "Actor Object Reference")))

(event `self.Collision Sphere.OnComponentBeginOverlap`
  (params (OverlappedComponent :type "PrimitiveComponent Object Reference") (OtherActor :type "Actor Object Reference") (OtherComp :type "PrimitiveComponent Object Reference") (OtherBodyIndex :type Integer) (bFromSweep :type Boolean) (SweepResult :type "HitResult Structure (by ref)"))
  ;[1 1 1] Detection
  (bind _asbp_enemi_parent (cast `/Game/Bleuprints/Enemies/BP_EnemiParent` OtherActor))
  (`KismetArrayLibrary.Array_Add` (`self.Tagert In Range`) _asbp_enemi_parent)
  (`/Engine/EditorBlueprintResources/StandardMacros.IsValid` (`self.Target Detected`)
    (:`Is Not Valid`
      (`self.Select Target`))))

(event `Begin Aim`
  ;[1 1 1] Aim
  (`|ExecutionSequence`
    (:`then_0`
      (goto _label :!via `Open`))
    (:`then_1`
      (`/Engine/EditorBlueprintResources/StandardMacros.Gate` true :!label _label
        (:`Exit`
          (`/Engine/EditorBlueprintResources/StandardMacros.IsValid` (`self.Target Detected`)
            (:`Is Valid`
              (`self.Cancel Aim`)
              (`self.Reset Aim`))))))))

(event `Continue Aim`
  ;[1 1 1] Aim
  (`/Engine/EditorBlueprintResources/StandardMacros.IsValid` (`self.Target Detected`)
    (:`Is Valid`
      (goto _label))
    (:`Is Not Valid`
      (goto _label :!via `Close`))))

(event `self.Collision Sphere.OnComponentEndOverlap`
  (params (OverlappedComponent :type "PrimitiveComponent Object Reference") (OtherActor :type "Actor Object Reference") (OtherComp :type "PrimitiveComponent Object Reference") (OtherBodyIndex :type Integer))
  (bind _tagert_in_range (`self.Tagert In Range`))
  ;[1 1 1] Detection
  (bind _asbp_enemi_parent (cast `/Game/Bleuprints/Enemies/BP_EnemiParent` OtherActor))
  (if (`KismetArrayLibrary.Array_Contains` _tagert_in_range _asbp_enemi_parent)
    (`KismetArrayLibrary.Array_RemoveItem` _tagert_in_range _asbp_enemi_parent)
    (if (== (`self.Target Detected`) _asbp_enemi_parent)
      (set `self.Target Detected` null)
      (`self.Select Target`))))

(event `Cancel Aim`
  ;[1 1 1] Aim
  (goto _label :!via `Close`))

(event `Select Target`
  (bind _tagert_in_range (`self.Tagert In Range`))
  ;[1 1 1] Selection
  (if (`KismetArrayLibrary.Array_IsValidIndex` _tagert_in_range)
    (set `self.Target Detected` (`|GetArrayItem` _tagert_in_range (`KismetMathLibrary.RandomIntegerInRange` 0 (`KismetArrayLibrary.Array_LastIndex` _tagert_in_range))))
    (`self.Begin Aim`)
    (else
      (`self.Reset Aim`))))

(event `Reset Aim`
  (`|ExecutionSequence`
    (:`then_0`
      (goto _label_2 :!via `Open`))
    (:`then_1`
      (`/Engine/EditorBlueprintResources/StandardMacros.Gate` true :!label _label_2
        (:`Exit`
          (`/Engine/EditorBlueprintResources/StandardMacros.IsValid` (`self.Target Detected`)
            (:`Is Valid`
              (`self.Stop Reset Aim`))))))))

(event `Continue Reset Aim`)

(event `Stop Reset Aim`)

(fn `Shoot`
  (bind _arrow (`self.Arrow`))
  (`|SpawnActorFromClass` "/Game/Bleuprints/Projectiles/BP_Devin_Spell.BP_Devin_Spell_C" (`KismetMathLibrary.MakeTransform` (`SceneComponent.K2_GetComponentLocation` _arrow) (`SceneComponent.K2_GetComponentRotation` _arrow)) "Undefined" "OverrideRootScale" null null))

(fn `UserConstructionScript`)