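; Enemy spawner that spawns pirates at its own location, facing along its Arrow component, with a spawn particle effect.
; Tick runs through a random Delay between Min and Max, so spawns repeat at irregular intervals.
; It spawns only BP_Pirate01 until the player's Minutes counter reaches one, then resets the delay range and randomly picks among three pirate classes.
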(event `self.ReceiveBeginPlay`
  ;[1 1 1] Spawn diffrent pirates
  (bind _asbp_player (cast `/Game/Bleuprints/Player/BP_Player` (`GameplayStatics.GetPlayerCharacter` 0)))
  (set `self.Player Ref` _asbp_player))

(event `self.ReceiveTick`
  (params (DeltaSeconds :type "Float (single-precision)"))
  ;[1 1 1] Spawn diffrent pirates
  (`KismetSystemLibrary.Delay` (`KismetMathLibrary.RandomFloatInRange` (`self.Min`) (`self.Max`)))
  (if (>= (`/Game/Bleuprints/Player/BP_Player.Minutes` (`self.Player Ref`)) 1)
    (set `self.Min` 2.0)
    (set `self.Max` 13.0)
    (if (<= (`KismetMathLibrary.RandomFloatInRange` 0.0 10.0) 3.3)
      (`self.Spawn_Pirates` "/Game/Bleuprints/Enemies/Pirates/BP_Pirate01.BP_Pirate01_C")
      (elif (>= (`/Game/Bleuprints/Player/BP_Player.Minutes` (`self.Player Ref`)) 1)
        (if (<= (`KismetMathLibrary.RandomFloatInRange` 0.0 7.0) 3.3)
          (`self.Spawn_Pirates` "/Game/Bleuprints/Enemies/Pirates/BP_Pirate02.BP_Pirate02_C")
          (else
            (`self.Spawn_Pirates` "/Game/Bleuprints/Enemies/Pirates/BP_Pirate03.BP_Pirate03_C")))
        (else
          (`self.Spawn_Pirates` "/Game/Bleuprints/Enemies/Pirates/BP_Pirate02.BP_Pirate02_C"))))
    (else
      (`self.Spawn_Pirates` "/Game/Bleuprints/Enemies/Pirates/BP_Pirate01.BP_Pirate01_C"))))

(fn `Spawn_Pirates`
  (params (Class :type "Actor Class Reference"))
  (bind (_returnvalue_x _returnvalue_y) (`KismetMathLibrary.BreakVector` (`SceneComponent.K2_GetComponentLocation` (`self.DefaultSceneRoot`))))
  (`|SpawnActorFromClass` Class (`KismetMathLibrary.MakeTransform` (`SceneComponent.K2_GetComponentLocation` (`self.DefaultSceneRoot`)) (`KismetMathLibrary.Conv_VectorToRotator` (`SceneComponent.GetForwardVector` (`self.Arrow`)))) "Undefined" "OverrideRootScale" null null)
  (`GameplayStatics.SpawnEmitterAtLocation` "/Game/Polygon/PolygonPirates/ParticleFX/P_FX_EnemySpawn.P_FX_EnemySpawn" (`KismetMathLibrary.MakeVector` _returnvalue_x _returnvalue_y 20.0)))

(fn `UserConstructionScript`)