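; BP_Demon is an enemy that travels along a spline path and is destroyed when damage depletes its Health.
; On BeginPlay it picks one of the first two BP_SplinePath actors at random, then starts Move.
; A timeline with play rate set by TimeToComplite lerps distance over the spline's length to set world location.
; Rotation always samples the spline's start in local space, so it does not follow the curve.
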(event `self.ReceiveBeginPlay`
  ;[1 1 1] Choose a Random Spline
  (bind _outactors (`GameplayStatics.GetAllActorsOfClass` "/Game/Bleuprints/BP_SplinePath.BP_SplinePath_C"))
  (set `self.SplineRef` (`|GetArrayItem` _outactors (`KismetMathLibrary.RandomIntegerInRange` 0 1)))
  (`self.Move`))

(event `Move`
  (bind _spline (`/Game/Bleuprints/BP_SplinePath.Spline` (`self.SplineRef`)))
  ;[1 1 1] Follow The Splin
  (`TimelineComponent.SetPlayRate` (`self.Move T`) (/ 1.0 (`self.TimeToComplite`)))
  (bind (_direction _movetrack) (`Timeline|Move T`)
    (:`Update`
      (`self.K2_SetActorTransform` (`KismetMathLibrary.MakeTransform` (`SplineComponent.GetLocationAtDistanceAlongSpline` _spline (`KismetMathLibrary.Lerp` 0.0 (`SplineComponent.GetSplineLength` (`/Game/Bleuprints/BP_SplinePath.Spline` (`self.SplineRef`))) _movetrack) "World") (`SplineComponent.GetRotationAtDistanceAlongSpline` _spline 0.0 "Local"))))))

(event `TakeDamage`
  (params (Damage :type "Float (double-precision)"))
  ;[1 1 1] Take Damage
  (set `self.Health` (- (`self.Health`) Damage))
  (if (<= (`self.Health`) 0.0)
    (`self.K2_DestroyActor`)))

(fn `UserConstructionScript`)