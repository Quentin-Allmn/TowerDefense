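; BP_Pirate01 is an enemy that travels along a randomly chosen BP_SplinePath and can be killed by spells.
; On BeginPlay it picks the path, then a timeline scaled by TimeToComplite moves it along the spline's length.
; Rotation is sampled only at the spline's start in local space, so it does not follow the curve.
; Capsule hits from Druid or Devin spells subtract their damage from health, destroying the pirate at zero.
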(event `self.ReceiveBeginPlay`
  ;[1 1 1] Choose a Random Spline
  (bind _outactors (`GameplayStatics.GetAllActorsOfClass` "/Game/Bleuprints/BP_SplinePath.BP_SplinePath_C"))
  (set `self.SplineRef` (`|GetArrayItem` _outactors (`KismetMathLibrary.RandomIntegerInRange` 0 (`KismetArrayLibrary.Array_LastIndex` _outactors))))
  (`self.Move`))

(event `Move`
  (bind _spline (`/Game/Bleuprints/BP_SplinePath.Spline` (`self.SplineRef`)))
  ;[1 1 1] Follow The Splin
  (`TimelineComponent.SetPlayRate` (`self.Timeline_Move`) (/ 1.0 (`self.TimeToComplite`)))
  (bind (_direction _movetrack) (`Timeline|Timeline_Move`)
    (:`Update`
      (`self.K2_SetActorTransform` (`KismetMathLibrary.MakeTransform` (`SplineComponent.GetLocationAtDistanceAlongSpline` _spline (`KismetMathLibrary.Lerp` 0.0 (`SplineComponent.GetSplineLength` (`/Game/Bleuprints/BP_SplinePath.Spline` (`self.SplineRef`))) _movetrack) "World") (`SplineComponent.GetRotationAtDistanceAlongSpline` _spline 0.0 "Local"))))))

(event `TakeDamage`
  (params (Damage :type "Float (double-precision)"))
  ;[1 1 1] Take Damage
  (set `self.Heatlth` (- (`self.Heatlth`) Damage))
  (if (<= (`self.Heatlth`) 0.0)
    (`self.K2_DestroyActor`)))

(event `self.Capsule_0.OnComponentHit`
  (params (HitComponent :type "PrimitiveComponent Object Reference") (OtherActor :type "Actor Object Reference") (OtherComp :type "PrimitiveComponent Object Reference") (NormalImpulse :type "Vector Structure") (Hit :type "HitResult Structure (by ref)"))
  (bind _asbp_druid_spell (cast `/Game/Bleuprints/Projectiles/BP_Druid_Spell` OtherActor)
    (:`then`
      (`self.TakeDamage` (`/Game/Bleuprints/Projectiles/BP_Druid_Spell.Damage` _asbp_druid_spell)))
    (:`CastFailed`
      (bind _asbp_devin_spell (cast `/Game/Bleuprints/Projectiles/BP_Devin_Spell` OtherActor))
      (`self.TakeDamage` (`/Game/Bleuprints/Projectiles/BP_Devin_Spell.Damage` _asbp_devin_spell)))))

(fn `UserConstructionScript`)