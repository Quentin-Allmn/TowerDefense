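; Minecart on a BP_Rail_2 spline that serves as a movable platform for cannon towers.
; On BeginPlay it picks a rail by index and places itself at a random spline point at fixed height.
; ChekCube maps two button cubes to up and down moves, which step the point index within hard-coded limits, play a sound and snap the cart there.
; Two attach functions spawn either cannon type on the cart with placement particles and set HaveTower.
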(event `self.ReceiveBeginPlay`
  (bind _returnvalue (`KismetMathLibrary.RandomIntegerInRange` 0 (`/Game/Bleuprints/Rails/BP_Rail_2.Spline Point` (`self.As BP Rail 2`))))
  (bind _returnvalue_2 (`SplineComponent.GetTransformAtSplinePoint` (`/Game/Bleuprints/Rails/BP_Rail_2.Spline` (`self.As BP Rail 2`)) _returnvalue "World" false))
  ;[1 1 1] Get Rail's Points
  (set `self.HaveTower` false)
  (bind _outactors (`GameplayStatics.GetAllActorsOfClass` "/Game/Bleuprints/Rails/BP_Rail_2.BP_Rail_2_C"))
  (bind _asbp_rail_2 (cast `/Game/Bleuprints/Rails/BP_Rail_2` (`|GetArrayItem` _outactors (`self.Index`))))
  (set `self.As BP Rail 2` _asbp_rail_2)
  (set `self.Poitn Index` _returnvalue)
  (`SceneComponent.K2_SetWorldTransform` (`self.DefaultSceneRoot`) (`KismetMathLibrary.MakeTransform` (`KismetMathLibrary.MakeVector` (.x (.location _returnvalue_2)) (.y (.location _returnvalue_2)) 40.0)) false false))

(event `Set Cart Position`
  (bind _returnvalue (`SplineComponent.GetTransformAtSplinePoint` (`/Game/Bleuprints/Rails/BP_Rail_2.Spline` (`self.As BP Rail 2`)) (`self.Poitn Index`) "World" false))
  ;[1 1 1] Set cart Position
  (`SceneComponent.K2_SetWorldTransform` (`self.DefaultSceneRoot`) (`KismetMathLibrary.MakeTransform` (`KismetMathLibrary.MakeVector` (.x (.location _returnvalue)) (.y (.location _returnvalue)) 40.0)) false false))

(event `Move Cart Down`
  ;[1 1 1] Move Cart by Direction
  (if (< (`self.Poitn Index`) 1)
    (set `self.Poitn Index` (+ (`self.Poitn Index`) 1))
    (`GameplayStatics.PlaySoundAtLocation` "/Game/Audio/mixkit-bed-pillow-hit-the-mattress-1901.mixkit-bed-pillow-hit-the-mattress-1901" (`SceneComponent.K2_GetComponentLocation` (`self.DefaultSceneRoot`)) (struct) 1.0 1.0 0.0 null null null null)
    (`self.Set Cart Position`)))

(event `MoveCart Up`
  ;[1 1 1] Move Cart by Direction
  (if (> (`self.Poitn Index`) 0)
    (set `self.Poitn Index` (- (`self.Poitn Index`) 1))
    (`GameplayStatics.PlaySoundAtLocation` "/Game/Audio/mixkit-bed-pillow-hit-the-mattress-1901.mixkit-bed-pillow-hit-the-mattress-1901" (`SceneComponent.K2_GetComponentLocation` (`self.DefaultSceneRoot`)) (struct) 1.0 1.0 0.0 null null null null)
    (`self.Set Cart Position`)))

(event `Chek Cube`
  (params (Asset :type "Object Object Reference"))
  ;[1 1 1] Check Cube
  (if (== (`self.Cube6`) Asset)
    (`self.MoveCart Up`)
    (elif (== (`self.Cube5`) Asset)
      (`self.Move Cart Down`))))

(fn `Attach_Cannon01`
  (bind _returnvalue (`SceneComponent.K2_GetComponentLocation` (`self.Cube`)))
  (bind _returnvalue_2 (`|SpawnActorFromClass` "/Game/Bleuprints/Towers/BP_Cannon.BP_Cannon_C" (`KismetMathLibrary.MakeTransform` _returnvalue (struct :`Yaw` 90.0)) "Undefined" "OverrideRootScale" null null))
  (`self.K2_AttachToActor` _returnvalue_2 self "None" "KeepWorld" "KeepWorld" "KeepWorld" true)
  (`GameplayStatics.SpawnEmitterAtLocation` "/Game/Polygon/PolygonPirates/ParticleFX/P_FX_TowerPlacement.P_FX_TowerPlacement" _returnvalue)
  (set `self.HaveTower` true))

(fn `Attach_Cannon02`
  (bind _returnvalue (`SceneComponent.K2_GetComponentLocation` (`self.Cube`)))
  (bind _returnvalue_2 (`|SpawnActorFromClass` "/Game/Bleuprints/Towers/BP_Cannon02.BP_Cannon02_C" (`KismetMathLibrary.MakeTransform` _returnvalue (struct :`Yaw` 90.0)) "Undefined" "OverrideRootScale" null null))
  (`self.K2_AttachToActor` _returnvalue_2 self "None" "KeepWorld" "KeepWorld" "KeepWorld" true)
  (`GameplayStatics.SpawnEmitterAtLocation` "/Game/Polygon/PolygonPirates/ParticleFX/P_FX_TowerPlacement.P_FX_TowerPlacement" _returnvalue)
  (set `self.HaveTower` true))

(fn `UserConstructionScript`)