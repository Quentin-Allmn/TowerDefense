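; Minecart actor that sits on a BP_Rail spline and serves as a movable mount for cannon towers.
; On BeginPlay it picks a rail by Index and snaps to a random spline point at fixed height.
; CheckCube matches a passed-in cube to step the cart up or down between points, with bounds and a sound.
; Two attach functions spawn and parent either cannon type with a placement effect, setting HaveTower.
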(event `self.ReceiveBeginPlay`
  (bind _rail_ref (`self.Rail Ref`))
  (bind _returnvalue (`KismetMathLibrary.RandomIntegerInRange` 0 (`/Game/Bleuprints/Rails/BP_Rail.Spline Point` _rail_ref)))
  (bind _returnvalue_2 (`SplineComponent.GetTransformAtSplinePoint` (`/Game/Bleuprints/Rails/BP_Rail.Spline` _rail_ref) _returnvalue "World" false))
  (set `self.HaveTower` false)
  (bind _outactors (`GameplayStatics.GetAllActorsOfClass` "/Game/Bleuprints/Rails/BP_Rail.BP_Rail_C"))
  (bind _asbp_rail (cast `/Game/Bleuprints/Rails/BP_Rail` (`|GetArrayItem` _outactors (`self.Index`))))
  (set `self.Rail Ref` _asbp_rail)
  (set `self.Poitn Index` _returnvalue)
  (`SceneComponent.K2_SetWorldTransform` (`self.DefaultSceneRoot`) (`KismetMathLibrary.MakeTransform` (`KismetMathLibrary.MakeVector` (.x (.location _returnvalue_2)) (.y (.location _returnvalue_2)) 40.0)) false false))

(event `Set Cart Position`
  (bind _returnvalue (`SplineComponent.GetTransformAtSplinePoint` (`/Game/Bleuprints/Rails/BP_Rail.Spline` (`self.Rail Ref`)) (`self.Poitn Index`) "World" false))
  (`SceneComponent.K2_SetWorldTransform` (`self.DefaultSceneRoot`) (`KismetMathLibrary.MakeTransform` (`KismetMathLibrary.MakeVector` (.x (.location _returnvalue)) (.y (.location _returnvalue)) 40.0)) false false))

(event `MoveCart Up`
  (if (< (`self.Poitn Index`) 3)
    (set `self.Poitn Index` (+ (`self.Poitn Index`) 1))
    (`GameplayStatics.PlaySoundAtLocation` "/Game/Audio/mixkit-bed-pillow-hit-the-mattress-1901.mixkit-bed-pillow-hit-the-mattress-1901" (`SceneComponent.K2_GetComponentLocation` (`self.DefaultSceneRoot`)) (struct) 1.0 1.0 0.0 null null null null)
    (`self.Set Cart Position`)))

(event `Move Cart Down`
  (if (> (`self.Poitn Index`) 0)
    (set `self.Poitn Index` (- (`self.Poitn Index`) 1))
    (`GameplayStatics.PlaySoundAtLocation` "/Game/Audio/mixkit-bed-pillow-hit-the-mattress-1901.mixkit-bed-pillow-hit-the-mattress-1901" (`SceneComponent.K2_GetComponentLocation` (`self.DefaultSceneRoot`)) (struct) 1.0 1.0 0.0 null null null null)
    (`self.Set Cart Position`)))

(event `Check Cube`
  (params (Asset :type "Object Object Reference"))
  (if (== (`self.Cube6`) Asset)
    (`self.MoveCart Up`)
    (elif (== (`self.Cube5`) Asset)
      (`self.Move Cart Down`)
      (else
        (`KismetSystemLibrary.PrintString` "False")))))

(fn `Attach_Cannon01`
  (bind _returnvalue (`SceneComponent.K2_GetComponentLocation` (`self.Cube`)))
  (bind _returnvalue_2 (`|SpawnActorFromClass` "/Game/Bleuprints/Towers/BP_Cannon.BP_Cannon_C" (`KismetMathLibrary.MakeTransform` _returnvalue (struct :`Yaw` 90.0)) "Undefined" "OverrideRootScale" null null))
  (`self.K2_AttachToActor` _returnvalue_2 self "None" "KeepWorld" "KeepWorld" "KeepWorld" true)
  (`GameplayStatics.SpawnEmitterAtLocation` "/Game/Polygon/PolygonPirates/ParticleFX/P_FX_TowerPlacement.P_FX_TowerPlacement" _returnvalue)
  (set `self.HaveTower` true))

(fn `Attach_Cannon02`
  (bind _returnvalue (`SceneComponent.K2_GetComponentLocation` (`self.Cube`)))
  (bind _returnvalue_2 (`|SpawnActorFromClass` "/Game/Bleuprints/Towers/BP_Cannon02.BP_Cannon02_C" (`KismetMathLibrary.MakeTransform` _returnvalue (struct :`Yaw` 90.0)) "Undefined" "OverrideRootScale" null null))
  (`self.K2_AttachToActor` _returnvalue_2 self "None" "KeepWorld" "KeepWorld" "KeepWorld" true)
  (`GameplayStatics.SpawnEmitterAtLocation` "/Game/Polygon/PolygonPirates/ParticleFX/P_FX_TowerPlacement.P_FX_TowerPlacement" _returnvalue)
  (set `self.HaveTower` true))

(fn `UserConstructionScript`)