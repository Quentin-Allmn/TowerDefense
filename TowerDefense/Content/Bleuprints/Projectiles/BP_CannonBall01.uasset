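; Cannonball projectile that damages pirate characters on contact and destroys itself after four seconds if it hits none.
; Each Tick, a very short Visibility line trace runs forward from the Arrow component.
; The hit actor is tested through chained casts to the three pirate Blueprints, calling TakeDamage on a match.
; Only pirate hits trigger the shared impact particle, sound and destruction; other hits are ignored.
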(event `self.ReceiveBeginPlay`
  (`KismetSystemLibrary.Delay` 4.0)
  (`self.K2_DestroyActor`))

(event `self.ReceiveTick`
  (params (DeltaSeconds :type "Float (single-precision)"))
  (bind _arrow (`self.Arrow`))
  (bind _returnvalue (`SceneComponent.K2_GetComponentLocation` _arrow))
  (bind _outhit (`KismetSystemLibrary.LineTraceSingle` _returnvalue (+ _returnvalue (* (`KismetMathLibrary.GetForwardVector` (`SceneComponent.K2_GetComponentRotation` _arrow)) 1.0)) "TraceTypeQuery1"))
  (bind (_bblockinghit _binitialoverlap _time _distance _location _impactpoint _normal _impactnormal _physmat _hitactor) (`GameplayStatics.BreakHitResult` _outhit))
  (bind _asbp_pirate_01 (cast `/Game/Bleuprints/Enemies/Pirates/BP_Pirate01` _hitactor)
    (:`then`
      (`/Game/Bleuprints/Enemies/Pirates/BP_Pirate01.TakeDamage` _asbp_pirate_01 (`self.Damage`)))
    (:`CastFailed`
      (bind _asbp_pirate_02 (cast `/Game/Bleuprints/Enemies/Pirates/BP_Pirate02` _hitactor)
        (:`then`
          (`/Game/Bleuprints/Enemies/Pirates/BP_Pirate02.TakeDamage` _asbp_pirate_02 (`self.Damage`)))
        (:`CastFailed`
          (bind _asbp_pirate_03 (cast `/Game/Bleuprints/Enemies/Pirates/BP_Pirate03` _hitactor))
          (`/Game/Bleuprints/Enemies/Pirates/BP_Pirate03.TakeDamage` _asbp_pirate_03 (`self.Damage`))))))
  (`GameplayStatics.SpawnEmitterAtLocation` "/Game/Polygon/PolygonPirates/ParticleFX/P_FX_Impact.P_FX_Impact" _impactpoint)
  (`GameplayStatics.PlaySoundAtLocation` "/Game/Audio/FRWKRec_Petard_a_meche_2__ID_1138__LS.FRWKRec_Petard_a_meche_2__ID_1138__LS" _impactpoint (struct) 1.0 1.0 0.0 null null null null)
  (`self.K2_DestroyActor`))

(fn `UserConstructionScript`)