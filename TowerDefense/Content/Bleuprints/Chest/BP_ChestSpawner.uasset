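; BP_ChestSpawner repeatedly spawns BP_Chest actors at random spawn points in the level.
; On BeginPlay it caches every BP_ChestSpanwPoint actor in an array.
; Tick drives a Delay of random length between Min and Max, which acts as a repeating timer.
; Each completed delay spawns a chest at a random cached point's location, with no check for existing chests.
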(event `self.ReceiveBeginPlay`
  ;[1 1 1] Get Spawn points
  (bind _outactors (`GameplayStatics.GetAllActorsOfClass` "/Game/Bleuprints/Chest/BP_ChestSpanwPoint.BP_ChestSpanwPoint_C"))
  (set `self.ChestPoint Ref` _outactors))

(event `self.ReceiveTick`
  (params (DeltaSeconds :type "Float (single-precision)"))
  (bind _chestpoint_ref (`self.ChestPoint Ref`))
  ;[1 1 1] Spawn Chest at random point
  (`KismetSystemLibrary.Delay` (`KismetMathLibrary.RandomFloatInRange` (`self.Min`) (`self.Max`)))
  (`|SpawnActorFromClass` "/Game/Bleuprints/Chest/BP_Chest.BP_Chest_C" (`KismetMathLibrary.Conv_VectorToTransform` (`SceneComponent.K2_GetComponentLocation` (`/Game/Bleuprints/Chest/BP_ChestSpanwPoint.DefaultSceneRoot` (`|GetArrayItem` _chestpoint_ref (`KismetMathLibrary.RandomIntegerInRange` 0 (`KismetArrayLibrary.Array_LastIndex` _chestpoint_ref)))))) "Undefined" "OverrideRootScale" null null))

(fn `UserConstructionScript`)