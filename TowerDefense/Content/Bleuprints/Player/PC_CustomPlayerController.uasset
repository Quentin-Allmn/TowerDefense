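; Player controller for tower placement that shows the interface widget and mouse cursor and handles clicks on mana and towers.
; Two placement events spawn a Druid or Soothsayer, which Tick moves to the cursor's visibility-trace hit, with a debug sphere, except over one concrete base.
; Releasing left mouse ends placement and refreshes the player's mana.
; Outside placement, clicking collects mana or upgrades a Druid.
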(event `Key|LeftMouseButton`
  (params (Key :type "Key Structure"))
  (bind _hitresult (`self.GetHitResultUnderCursorByChannel` "TraceTypeQuery1"))
  (:`Pressed`
    (if (`self.Placing`)
      _
      (elif (`GameplayStatics.BreakHitResult` _hitresult)
        (bind _asbp_mana (cast `/Game/Bleuprints/BP_Mana` (`.HitActor` (`GameplayStatics.BreakHitResult` _hitresult)))
          (:`then`
            (`/Game/Bleuprints/BP_Mana.Click On Mana` _asbp_mana)
            (`/Game/Bleuprints/Player/BP_Player.Add Mana` (`self.Player Ref`)))
          (:`CastFailed`
            (bind _asbp_druid (cast `/Game/Bleuprints/Towers/BP_Druid` (`.HitActor` (`GameplayStatics.BreakHitResult` _hitresult)))
              (:`then`
                (`/Game/Bleuprints/Towers/BP_Druid.Upgrade` _asbp_druid))
              (:`CastFailed`
                (`KismetSystemLibrary.PrintString` "Hello"))))))))
  (:`Released`
    (set `self.Placing` false)
    (`/Game/Bleuprints/Player/BP_Player.Call_Mana_Refresh` (`self.Player Ref`))))

(event `self.ReceiveTick`
  (params (DeltaSeconds :type "Float (single-precision)"))
  (bind _hitresult (`self.GetHitResultUnderCursorByChannel` "TraceTypeQuery1"))
  ;[1 1 1] Tower Placement
  (if (`self.Placing`)
    (if (`GameplayStatics.BreakHitResult` _hitresult)
      (if (not (== (`.HitActor` (`GameplayStatics.BreakHitResult` _hitresult)) "/Game/Polygon/PolygonTown/Meshes/Environment/SM_Env_Concrete_Base_01.SM_Env_Concrete_Base_01"))
        (`KismetSystemLibrary.DrawDebugSphere` (`.ImpactPoint` (`GameplayStatics.BreakHitResult` _hitresult)) 100.0 12 (struct :`R` 1.0 :`B` 0.113573 :`A` 1.0))
        (switch `int` (`self.Tower_index`)
          (:`0`
            (`self.K2_SetActorLocation` (stale `EventPlacingMode` _returnvalue) (`.ImpactPoint` (`GameplayStatics.BreakHitResult` _hitresult)) false false))
          (:`1`
            (`self.K2_SetActorLocation` (stale `PlacingDevin` _returnvalue) (`.ImpactPoint` (`GameplayStatics.BreakHitResult` _hitresult)) false false)))))))

(event `PlacingDevin`
  (set `self.Tower_index` 1)
  (if (not (`self.Placing`))
    (set `self.Placing` true)
    (bind _returnvalue (`|SpawnActorFromClass` "/Game/Bleuprints/Towers/BP_Soothsayer.BP_Soothsayer_C" (`KismetMathLibrary.MakeTransform` (0.0 0.0 0.0)) "Undefined" "OverrideRootScale" null null))
    (set `self.CurrentSpawned` _returnvalue)
    (`PrimitiveComponent.SetCollisionResponseToChannel` (`/Game/Bleuprints/Towers/BP_Soothsayer.SkeletalMesh` _returnvalue) "ECC_Visibility" "ECR_Block")))

(event `EventPlacingMode`
  ;[1 1 1] Tower Placement
  (set `self.Tower_index` 0)
  (if (not (`self.Placing`))
    (set `self.Placing` true)
    (bind _returnvalue (`|SpawnActorFromClass` "/Game/Bleuprints/Towers/BP_Druid.BP_Druid_C" (`KismetMathLibrary.MakeTransform` (0.0 0.0 0.0)) "Undefined" "OverrideRootScale" null null))
    (set `self.CurrentSpawned` _returnvalue)
    (`PrimitiveComponent.SetCollisionResponseToChannel` (`/Game/Bleuprints/Towers/BP_Druid.SkeletalMesh` _returnvalue) "ECC_Visibility" "ECR_Block")))

(event `self.ReceiveBeginPlay`
  ;[1 1 1] Widgets
  (bind _returnvalue (`|CreateWidget` "/Game/Bleuprints/UI/WG_Interface.WG_Interface_C" null self))
  (bind _output_get (set `self.Interface Ref` _returnvalue))
  (`UserWidget.AddToViewport` _output_get 0)
  (set `self.bShowMouseCursor` true)
  (bind _asbp_player (cast `/Game/Bleuprints/Player/BP_Player` (`GameplayStatics.GetPlayerCharacter` 0)))
  (set `self.Player Ref` _asbp_player))

(fn `UserConstructionScript`)