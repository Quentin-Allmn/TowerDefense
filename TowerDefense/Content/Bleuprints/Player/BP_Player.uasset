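; BP_Player is the player Blueprint that owns the HUD widget, a mana total and an elapsed-time counter.
; BeginPlay enables input and adds a WG_Player widget to the viewport, which AddMana and CallManaRefresh update with the current mana.
; Tick uses a one-second Delay as a clock, incrementing Seconds and rolling over into Minutes when it reaches 59.
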(event `self.ReceiveBeginPlay`
  (`self.EnableInput` (`GameplayStatics.GetPlayerController` 0))
  (bind _returnvalue (`|CreateWidget` "/Game/Bleuprints/UI/WG_Player.WG_Player_C"))
  (bind _output_get (set `self.UI Ref` _returnvalue))
  (`UserWidget.AddToViewport` _output_get 0))

(event `self.ReceiveTick`
  (params (DeltaSeconds :type "Float (single-precision)"))
  (`KismetSystemLibrary.Delay` 1.0)
  (set `self.Seconds` (+ (`self.Seconds`) 1))
  (if (== (`self.Seconds`) 59)
    (set `self.Minutes` (+ (`self.Minutes`) 1))
    (set `self.Seconds` 0)))

(fn `Add Mana`
  (set `self.Mana` (+ (`self.Mana`) (`self.Mana to Add`)))
  (`/Game/Bleuprints/UI/WG_Player.Refresh Mana` (`self.UI Ref`) (`KismetTextLibrary.Conv_IntToText` (`self.Mana`))))

(fn `Call_Mana_Refresh`
  (`/Game/Bleuprints/UI/WG_Player.Refresh Mana` (`self.UI Ref`) (`KismetTextLibrary.Conv_IntToText` (`self.Mana`))))

(fn `UserConstructionScript`)